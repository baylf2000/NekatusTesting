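; Sequence-puzzle door for ASA that opens when its linked buttons are pressed in the configured order, then auto-closes.
; After a startup delay, the server links buttons and indicators sharing its NetworkTag.
; Presses light indicators by group and advance the sequence; wrong presses reset it, and ReceiveButtonState can also open the door directly.
; DoorState replicates as a byte because bools replicate incorrectly in ASA; its OnRep drives client-only timeline movement.
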(event Custom|SetDoorVisual_Open
  (params (Instant :type Boolean))
  (bind _openlocation (Variables|Config|GetOpenLocation))
  (bind _openlocation_2 (Variables|Config|GetOpenLocation))
  ;[0.07329 0.84 0] Set the visual state of the door mesh to Open. Normally the "Instant" input variable would be false, allowing the door to open slowly over the time period configured in "DoorOpenSpeed" (in seconds). The "Instant" variable causes the door to instantly move to the open position.
  (Development|PrintString 0 "SetDoorVisual_Open")
  (if Instant ; Do it instantly, without timeline?
    (Transformation|SetRelativeLocation (Variables|Default|GetDoorMesh) (Math|Vector|MakeVector (.x _openlocation_2) (.y _openlocation_2) (.z _openlocation_2)) false false)
    (else
      (Components|Timeline|SetPlayRate (Variables|Default|GetTimeline_DoorOpen) (/ 1.0 (Variables|Config|GetDoorOpenSpeed))) ; Change timeline playback rate to match \nthe config variable "DoorOpenSpeed"
      (bind _dooropen (Timeline|Timeline_DoorOpen PlayFromStart)
        (:Update
          (Transformation|SetRelativeLocation (Variables|Default|GetDoorMesh) (Math|Vector|MakeVector (* (- (.x _openlocation) (.x (Variables|Config|GetClosedLocation))) _dooropen) (.y _openlocation) (.z _openlocation)) false false))
        (:Finished
          (Development|PrintString 0 "SetDoorVisual_Open - Finish Timeline"))))))

(event Custom|SetDoorVisual_Closed
  (params (Instant :type Boolean))
  (bind _closedlocation (Variables|Config|GetClosedLocation))
  (bind _closedlocation_2 (Variables|Config|GetClosedLocation))
  ;[1 1 1] Set the visual state of the door mesh to Closed. Normally the "Instant" input variable would be false, allowing the door to close slowly over the time period configured in "DoorCloseSpeed" (in seconds). The "Instant" variable causes the door to instantly move to the closed position.
  (Development|PrintString 0 "SetDoorVisual_Closed")
  (if Instant ; Do it instantly, without timeline?
    (Transformation|SetRelativeLocation (Variables|Default|GetDoorMesh) (Math|Vector|MakeVector (.x _closedlocation) (.y _closedlocation) (.z _closedlocation)) false false)
    (else
      (Components|Timeline|SetPlayRate (Variables|Default|GetTimeline_DoorClose) (/ 1.0 (Variables|Config|GetDoorCloseSpeed))) ; Change timeline playback rate to match \nthe config variable "DoorCloseSpeed"
      (bind _doorclose (Timeline|Timeline_DoorClose PlayFromStart)
        (:Update
          (Transformation|SetRelativeLocation (Variables|Default|GetDoorMesh) (Math|Vector|MakeVector (* (- (.x (Variables|Config|GetOpenLocation)) (.x _closedlocation_2)) _doorclose) (.y _closedlocation_2) (.z _closedlocation_2)) false false))
        (:Finished
          (Development|PrintString 0 "SetDoorVisual_Closed - Finish Timeline"))))))

(event EventBeginPlay
  (Utilities|FlowControl|Delay 0 5.0) ; Ensure buttons and indicators have time to\nload before searching.
  (Utilities|FlowControl|Sequence
    (:then_0
      ;[1 1 1] Server - Get references to the connected buttons and indicators for this area.
      (Networking|SwitchHasAuthority
        (:Authority
          (CallFunction|GetConnectedButtons)
          (CallFunction|GetConnectedIndicators))))))

(event EventNKButtonPress
  (params (DeviceID :type Byte :default 0) (GroupID :type Byte :default 0))
  (Development|PrintText self (Utilities|Text|FormatText "Event NK Button Press - DeviceID: {device}, GroupID: {group}" DeviceID GroupID))
  (CallFunction|ProcessButtonPress DeviceID GroupID))

(fn ConstructionScript)

(fn GetConnectedButtons
  ;[1 1 1] This finds all the buttons on the map with the custom tag that matches the one used for this door, and saves them in an array.
  ; It also registers itself with those buttons so that they know who their parent door is.
  (Utilities|Array|Clear (Variables|Default|GetConnectedButtons))
  (bind _outactors (Actor|GetAllActorsOfClasswithTag self "/NekatusTesting/Assets/BP_Nekatus_Button_01.BP_Nekatus_Button_01_C" (Variables|Config|GetNetworkTag)))
  (for _array_element _outactors
    (Utilities|IsValid _array_element
      (:Is%20Valid
        ;;[1 1 1] This adds the found button to an array that contains a struct which is made up of the button reference, the button's device id and the button's group id.
        (Default|ReceiveParentReference _array_element self)
        (Utilities|Array|Add (Variables|Default|GetConnectedButtons) (Utilities|Struct|MakeNK_Buttons_Struct _array_element (Variables|/NekatusTesting/Assets/BP_Nekatus_Button_01.BP_Nekatus_Button_01_C|GetDeviceID _array_element) (Variables|/NekatusTesting/Assets/BP_Nekatus_Button_01.BP_Nekatus_Button_01_C|GetGroupID _array_element))))))
  (Development|PrintText self (Utilities|Text|FormatText "Found and connected to {x} buttons." (Utilities|Array|Length (Variables|Default|GetConnectedButtons)))))

(fn GetConnectedIndicators
  ;[1 1 1] This finds all the indicators on the map with the custom tag that matches the "NetworkTag" variable, and saves them in an array.
  ; It also registers itself with those indicators so that they know who their parent door is.
  (Utilities|Array|Clear (Variables|Default|GetConnectedIndicators))
  (bind _outactors (Actor|GetAllActorsOfClasswithTag self "/NekatusTesting/Assets/BP_Nekatus_Indicator_01.BP_Nekatus_Indicator_01_C" (Variables|Config|GetNetworkTag)))
  (for _array_element _outactors
    (Utilities|IsValid _array_element
      (:Is%20Valid
        ;;[1 1 1] This adds the found indicator to an array that contains a struct which is made up of the indicator reference, the bindicator's device id and the indicator's group id.
        (Default|ReceiveParentReference _array_element)
        (Utilities|Array|Add (Variables|Default|GetConnectedIndicators) (Utilities|Struct|MakeNK_Indicators_Struct _array_element (Variables|/NekatusTesting/Assets/BP_Nekatus_Indicator_01.BP_Nekatus_Indicator_01_C|GetDeviceID _array_element) (Variables|/NekatusTesting/Assets/BP_Nekatus_Indicator_01.BP_Nekatus_Indicator_01_C|GetGroupID _array_element))))))
  (Development|PrintText self (Utilities|Text|FormatText "Found and connected to {x} indicators." (Utilities|Array|Length (Variables|Default|GetConnectedIndicators)))))

(fn ReceiveButtonState
  (params (ButtonID :type Byte) (ButtonState :type Byte))
  (bind _self self)
  (bind _state (CallFunction|NKBytetoState ButtonState _self))
  (Development|PrintText self (Utilities|Text|FormatText "ReceiveButtonState - ButtonID: {id}, State: {state}" ButtonID _state))
  (if _state
    (CallFunction|SetDoorStateOpen false 0.0)))

(fn SetVisualState
  (params (DoorIsOpen :type Boolean))
  ;[1 1 1] Use this function to do whatever is required to change the visual state of the door to either open or closed. This function will only be called on clients, so it should only change visual details.
  (Class|KismetSystemLibrary|CanRunCosmeticEvents self ; This node will only return "Yes" for clients,\nnot servers.
    (:Yes
      (Transformation|SetMobility (Variables|Default|GetDoorMesh) "Movable") ; WC have added something in C++ that sets mobility to static. \nNeed to change this manually back to moveable.
      (if DoorIsOpen
        (CallFunction|SetDoorVisualOpen false) ; Set the door mesh to the open position.
        (Development|PrintString 0 "SetVisualState - Open")
        (else
          (CallFunction|SetDoorVisualClosed false) ; Set the door mesh to the closed position.
          (Development|PrintString 0 "SetVisualState - Closed"))))))

(fn OnRepDoorState
  ;[1 1 1] This function is automatically called each time the "DoorState" variable changes value. It's run on the server and all relevant clients. In this situation it's used to change the visual state of clients to show the door as either open or closed.
  (Class|KismetSystemLibrary|CanRunCosmeticEvents self ; This node will only return "Yes" for clients,\nnot servers.
    (:Yes
      (Development|PrintString 0 "OnRepDoorState")
      (CallFunction|SetVisualState (CallFunction|NKBytetoState (Variables|Default|GetDoorState) self)))))

(fn SetDoorStateOpen
  (params (AutoClose :type Boolean) (AutoCloseTime :type Float%20%28double-precision%29))
  ;[1 1 1] Should only be called from Server. Converts the "true" boolean to a byte value which will be replicated and 'OnRep_DoorState' will run on server and all clients. A byte is used for replication as boolean values currently do not replicate correctly in ASA.
  ; Includes a bool option "AutoClose" which, if true, adds a timer to close the door again after x seconds, as supplied in the "AutoCloseTime" input variable.
  (Development|PrintString 0 "SetDoorState_Open")
  (Utilities|FlowControl|Sequence
    (:then_0
      (Variables|Default|SetDoorState (CallFunction|NKStatetoByte true self) true))
    (:then_1
      (if AutoClose
        (Utilities|Time|SetTimerbyFunctionName 0 "SetDoorState_Closed" AutoCloseTime)))))

(fn SetDoorStateClosed
  ;[1 1 1] Should only be called from Server. Converts the "false" boolean to a byte value which will be replicated and 'OnRep_DoorState' will run on server and all clients. A byte is used for replication as boolean values currently do not replicate correctly in ASA.
  (Development|PrintString 0 "SetDoorState_Closed")
  (Variables|Default|SetDoorState (CallFunction|NKStatetoByte false self) true))

(fn ProcessButtonPress
  (params (DeviceID :type Byte) (GroupID :type Byte))
  (Utilities|FlowControl|Sequence
    (:then_0
      (CallFunction|CheckGroup GroupID))
    (:then_1
      (if (CallFunction|IsNextButton DeviceID)
        (bind _sequencecomplete (CallFunction|MoveNextStep))
        (if _sequencecomplete
          (CallFunction|ResetSequence)
          (CallFunction|ProcessCompletion))
        (else
          (CallFunction|ResetSequence))))))

(fn IsNextButton
  (params (DeviceID :type Byte))
  ;[1 1 1] If the device ID of this button press matches the configured device ID of the current step in the configured sequence, then return true, otherwise false. Note: This is configured as a "pure" function which means it doesn't need the exec inputs and outputs when called.
  (return (== DeviceID (Utilities|Array|Get(acopy) (Variables|Config|GetButtonSequence) (Variables|Default|GetSequenceStep)))))

(fn MoveNextStep
  ;[1 1 1] If, after incrementing the step counter, it has the same number of steps as the configured "ButtonSequence" then the sequence must be correctly complete. If so return true, otherwise false. This function is **only** called once a button has been matched to the current deviceid in the configured sequence with the "IsNextButton" function.
  (bind _result (Math|Integer|IncrementInt (Variables|Default|GetSequenceStep))
    (:%20%20
      (return (== (Utilities|Array|Length (Variables|Config|GetButtonSequence)) _result)))))

(fn ProcessCompletion
  (CallFunction|AllIndicatorReset)
  (CallFunction|SetDoorStateOpen true (Variables|Config|GetAutoCloseTime)))

(fn ResetSequence
  (Variables|Default|SetSequenceStep 0)
  (CallFunction|AllIndicatorReset))

(fn CheckGroup
  (params (GroupID :type Byte))
  ;[1 1 1] Takes the supplied "GroupID" and loops through all the connected indicators to see if their GroupID matches. If there's a match, it activates that indicator.
  (for _array_element (Variables|Default|GetConnectedIndicators)
    (if (== GroupID (.GroupID (Utilities|Struct|BreakNK_Indicators_Struct _array_element)))
      (Utilities|IsValid (.IndicatorRef (Utilities|Struct|BreakNK_Indicators_Struct _array_element))
        (:Is%20Valid
          (CallFunction|SetIndicatorState true (.IndicatorRef (Utilities|Struct|BreakNK_Indicators_Struct _array_element)) 0.0) ; If the "ResetTime" is zero, the indicator will use \nits internal default reset time.
        )))))

(fn SetIndicatorState
  (params (IndicatorState :type Boolean) (DeviceRef :type Actor%20Object%20Reference) (ResetTime :type Float%20%28double-precision%29))
  ;[1 1 1] Using the supplied device reference, use the blueprint interface "NKSetIndicatorState" to tell the indicator to activate. Also supply the amount of time the indicator should wait until it resets.
  (Utilities|IsValid DeviceRef ; Always check a reference like this to \nensure it's valid, otherwise it could \ncrash the server.
    (:Is%20Valid
      (Class|InterfaceNekatusBDI|NKSetIndicatorState(Message) DeviceRef IndicatorState ResetTime))))

(fn AllIndicatorReset
  ;[1 1 1] Loop through all connected indicators and reset them.
  (for _array_element (Variables|Default|GetConnectedIndicators)
    (Utilities|IsValid (.IndicatorRef (Utilities|Struct|BreakNK_Indicators_Struct _array_element))
      (:Is%20Valid
        (CallFunction|SetIndicatorState false (.IndicatorRef (Utilities|Struct|BreakNK_Indicators_Struct _array_element)) 0.0)))))

(fn FullNetworkReset
  ;[1 1 1] This resets everything back to start. Door closed. All Indicators reset. Sequence back to first step. Add anything else here that needs to happen to restart the network.
  (Utilities|FlowControl|Sequence
    (:then_0
      (CallFunction|SetDoorStateClosed))
    (:then_1
      (for _array_element (Variables|Default|GetConnectedIndicators)
        (Utilities|IsValid (.IndicatorRef (Utilities|Struct|BreakNK_Indicators_Struct _array_element))
          (:Is%20Valid
            (CallFunction|SetIndicatorState false (.IndicatorRef (Utilities|Struct|BreakNK_Indicators_Struct _array_element)) 0.0)))))
    (:then_2
      (CallFunction|ResetSequence))))