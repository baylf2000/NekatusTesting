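; Networked push-button actor that players press through a multi-use "Press Button" entry to signal its parent door.
; The server handles the press, sends device and group IDs to the registered door through an interface, and resets the button on a timer.
; RepNotify ButtonState moves the mesh between rest and pressed positions on clients, forcing it Movable first.
; The construction script adds the network name as an actor tag.
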(event EventBeginPlay
  (LogicalStates|SetButtonState false) ; Make sure the button is not pressed by default.
)

(event Collision|EventActorBeginOverlap
  (params (OtherActor :type Actor%20Object%20Reference)))

(event EventTick
  (params (DeltaSeconds :type Float%20%28single-precision%29)))

(fn ConstructionScript
  ;[1 1 1] Use this to set the network tag at the earliest possible time
  (CallFunction|SetNetworkTag))

(fn BPGetMultiUseEntries
  (params (ForPC :type Player%20Controller%20Object%20Reference) (MultiUseEntries :type Array%20of%20Multi%20Use%20Entry%20Structures))
  ;[1 1 1] This is run on the client, and adds the multiuse menu option to the button actor for "Press Button", which should be the only option in this case. The corresponding function "BPTryMultiuse" will be called **on the server** when the player actions this option by pressing "E".
  (if (CallFunction|NKBytetoState (Variables|Running|GetButtonState) self)
    _
    (else
      (Utilities|Array|Add MultiUseEntries (Utilities|Struct|MakeMultiUseEntry 0 "Press Button" 12505 0 false false false false false false false false false false false false false false 0 false 0 "(B=175,G=175,R=175,A=255)" "(B=255,G=255,R=255,A=255)" 0.0 0.0 0 -1 -1 "/Game/PrimalEarth/CoreBlueprints/StatusIcons/HandHarvestYes.HandHarvestYes"))))
  (return MultiUseEntries))

(fn BPTryMultiUse
  (params (ForPC :type Player%20Controller%20Object%20Reference) (UseIndex :type Integer))
  ;[1 1 1] This is called on the SERVER when a player chooses a multiuse menu item. The "Use Index" is specified in the entry added in "BPGetMultiuseEntries". We use this variable to determine which option was chosen. In this case there should only be one option, but we'll check it anyway. Then we notify the connected door that this button was pressed in the "NotifyDoor" function, then change the RepNotify "ButtonState" variable in "SetButtonState". That will then call "OnRep_ButtonState" on all clients which will change the visual state of the button. A timer is added to do the reverse and reset the button state after x seconds. I also added a check to make sure the button isn't already in the pressed state. That should be impossible as the menu option is removed while the button is in the pressed state, but this is an additional check.
  (Utilities|FlowControl|Sequence
    (:then_0
      (if (== UseIndex 12505) ; Does the use index match that of the \n"Press Button" option we added.
        (if (not (CallFunction|NKBytetoState (Variables|Running|GetButtonState) self)) ; Is the button already pressed?
          (Development|PrintString 0 "BPTryMultiUse - Button Press")
          (CallFunction|NotifyDoor)
          (LogicalStates|SetButtonState true)
          (Utilities|Time|SetTimerbyFunctionName 0 "ResetButton" (Variables|Config|GetButtonResetTime)))))
    (:then_1
      (return true))))

(fn SetButtonState
  (params (IsPressed :type Boolean))
  (Variables|Running|SetButtonState (CallFunction|NKStatetoByte IsPressed self) true))

(fn ResetButton
  (Development|PrintString 0 "ResetButton")
  (LogicalStates|SetButtonState false))

(fn OnRepButtonState
  ;[1 1 1] This function is automatically called each time the "ButtonState" variable changes value. It's run on the server and all relevant clients. In this situation it's used to change the visual state of clients to show the button as either pressed or not pressed.
  (Class|KismetSystemLibrary|CanRunCosmeticEvents self ; This node will only return "Yes" for clients,\nnot servers.
    (:Yes
      (CallFunction|SetVisualState (CallFunction|NKBytetoState (Variables|Running|GetButtonState) self)))))

(fn SetVisualState
  (params (IsPressed :type Boolean))
  ;[1 1 1] Use this function to do whatever is required to change the visual state of the button to either pressed or not pressed. This function will only be called on clients, so it should only change visual details.
  (Class|KismetSystemLibrary|CanRunCosmeticEvents self ; This node will only return "Yes" for clients,\nnot servers.
    (:Yes
      (Transformation|SetMobility (Variables|Default|GetMyStaticMesh) "Movable") ; WC have added something in C++ that sets mobility to static. \nNeed to change this manually back to moveable.
      (if IsPressed
        (Transformation|SetRelativeLocation (Variables|Default|GetMyStaticMesh) (Variables|Config|GetPressedPosition) false false)
        (Development|PrintString 0 "SetVisualState - Pressed")
        (else
          (Transformation|SetRelativeLocation (Variables|Default|GetMyStaticMesh) (Variables|Config|GetRestPosition) false false)
          (Development|PrintString 0 "SetVisualState - Rest"))))))

(fn NotifyDoor
  (bind _parentdoor (Variables|Running|GetParentDoor))
  ;[1 1 1] Uses the Blueprint Interface "NKButtonPress" to signify to the door that a button has been pressed, passing the device id and group id of this button instance.
  (Utilities|IsValid _parentdoor ; Make sure the store reference to the parent is valid.
    (:Is%20Valid
      (Class|InterfaceNekatusBDI|NKButtonPress(Message) _parentdoor (Variables|Config|GetDeviceID) (Variables|Config|GetGroupID)) ; This is an blueprint interface function to signify a button press.
    )))

(fn ReceiveParentReference
  (params (ParentDoor :type Actor%20Object%20Reference))
  ;[1 1 1] This is just a function that will be called by the parent door at startup to register itself as the parent door. The reference is used later to notify the parent of a button press.
  (Utilities|IsValid ParentDoor
    (:Is%20Valid
      (Variables|Running|SetParentDoor ParentDoor)
      (Development|PrintString 0 "Received Parent Reference."))))

(fn SetNetworkTag
  (Utilities|Array|AddUnique (Variables|Default|GetTags) (Variables|Config|GetNetworkName)))