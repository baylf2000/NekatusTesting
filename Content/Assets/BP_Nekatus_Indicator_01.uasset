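; BP_Nekatus_Indicator_01 is a networked indicator light that a parent door drives, tagged with its NetworkName at construction.
; NKSetIndicatorState stores on/off as a byte and, when switching on, starts a timer that switches it off after IndicatorResetTime.
; OnRep_IndicatorState toggles the mesh material's EmissiveValue where cosmetic events can run.
; ReceiveParentReference is a hook for future use, as communication currently runs only from door to indicator.
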(event EventBeginPlay
  (Utilities|FlowControl|Sequence
    (:then_0
      (Networking|SwitchHasAuthority))
    (:then_1
      (Class|KismetSystemLibrary|CanRunCosmeticEvents self
        (:Yes
          (CallFunction|DisableIndicator))))))

(event Collision|EventActorBeginOverlap
  (params (OtherActor :type Actor%20Object%20Reference)))

(event EventTick
  (params (DeltaSeconds :type Float%20%28single-precision%29)))

(event EventNKSetIndicatorState
  (params (IndicatorState :type Boolean) (ResetTime :type Float%20%28double-precision%29))
  (Development|PrintString 0 (Utilities|String|Append "EventNKSetIndicatorState - State: " (Utilities|String|ToString(Boolean) IndicatorState)))
  (if IndicatorState
    (CallFunction|EnableIndictaor)
    (Utilities|Time|SetTimerbyFunctionName 0 "DisableIndicator" (Variables|Config|GetIndicatorResetTime))
    (else
      (CallFunction|DisableIndicator))))

(fn ConstructionScript
  (CallFunction|SetNetworkTag))

(fn ReceiveParentReference
  (params (ParentDoor :type Actor%20Object%20Reference))
  ;[1 1 1] This is just a function that will be called by the parent door at startup to register itself as the parent door. This may be used in future but is not required right now, as communication is from the parent door to the indicator only, not the other direction.
  (Utilities|IsValid ParentDoor
    (:Is%20Valid
      (Variables|Default|SetParentDoor ParentDoor))))

(fn SetVisualState
  (params (IndicatorEnabled :type Boolean))
  (bind _staticmesh (Variables|Default|GetStaticMesh))
  (if IndicatorEnabled
    (Rendering|Material|SetScalarParameterValueonMaterials _staticmesh "EmissiveValue" 5e+01)
    (else
      (Rendering|Material|SetScalarParameterValueonMaterials _staticmesh "EmissiveValue" 0.0))))

(fn OnRepIndicatorState
  (bind _self self)
  (bind _indicatorstate (Variables|Default|GetIndicatorState))
  (bind _state (CallFunction|NKBytetoState _indicatorstate _self))
  (Class|KismetSystemLibrary|CanRunCosmeticEvents self
    (:Yes
      (Development|PrintString 0 (Utilities|String|Append "OnRepIndicatorState - State: " (Utilities|String|ToString(Boolean) _state)))
      (CallFunction|SetVisualState _state))))

(fn EnableIndictaor
  (Variables|Default|SetIndicatorState (CallFunction|NKStatetoByte true self) true))

(fn DisableIndicator
  (Variables|Default|SetIndicatorState (CallFunction|NKStatetoByte false self) true))

(fn SetNetworkTag
  ;[1 1 1] This adds an actor tag equal to the configured "NetworkName"
  (Utilities|Array|AddUnique (Variables|Actor|GetTags) (Variables|Config|GetNetworkName)))